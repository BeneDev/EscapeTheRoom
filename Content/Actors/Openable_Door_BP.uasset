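; Openable door actor that swings open and closed when its OpenDoor component receives open or close requests.
; A DoorSwing timeline adds an animated yaw angle to the rotation cached at BeginPlay, and closing plays the same timeline in reverse.
; A timeline event track triggers the door lock sound at the door's location.
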(event `self.OpenDoor.OnOpenRequest`
  (bind (_direction _openangle) (`Timeline|Door Swing` :!label _label)
    (:`Update`
      (`self.K2_SetActorRotation` (`KismetMathLibrary.ComposeRotators` (`KismetMathLibrary.MakeRotator` 0.0 0.0 _openangle) (`self.InitialRotation`))))
    (:`Sound Timing`
      (`GameplayStatics.PlaySoundAtLocation` "/Game/SFX/door-lock.door-lock" (`self.K2_GetActorLocation`)))))

(event `self.OpenDoor.OnCloseRequest`
  (goto _label :!via `Reverse`))

(event `self.ReceiveBeginPlay`
  (set `self.InitialRotation` (`self.K2_GetActorRotation`)))

(fn `UserConstructionScript`)